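; BP_Quest is the base quest Blueprint in the quest system, meant to be subclassed for individual quests.
; On BeginPlay it constructs a root objective collection, stores it, populates its objectives and then activates it.
; The construct and populate functions act as override hooks, printing on-screen errors if the base versions run.
; A getter exposes the root objective collection.
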(event EventBeginPlay
  (bind _rootobjcollection (Private|ConstructRootObjectiveCollection))
  (bind _output_get (Variables|Private|SetRootObjectiveCollection _rootobjcollection))
  (Private|PopulateObjectives _output_get)
  (Default|ActivateObjective (Variables|Private|GetRootObjectiveCollection)))

(fn ConstructionScript)

(fn ConstructRootObjectiveCollection
  (Development|PrintString "ERROR: CREATE RootObjectiveCollection called for base class!" true true "(R=0.546875,G=0.000000,B=0.024653,A=1.000000)" 1e+01)
  (return 0))

(fn PopulateObjectives
  (params (RootObjCollection :type BP%20Obj%20Collection%20Object%20Reference))
  (Development|PrintString "ERROR: Populate Objectives called for base class!" true true "(R=0.546875,G=0.000000,B=0.024653,A=1.000000)" 1e+01))

(fn GetRootObjectiveCollection
  (return (Variables|Private|GetRootObjectiveCollection)))