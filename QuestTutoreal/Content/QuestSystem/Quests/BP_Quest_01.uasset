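; BP_Quest_01 defines the "A Long Way Home" quest, which has the player reach three destinations: GEEKBRAINS, SKILLBOX and NETOLOGY.
; ConstructRootObjectiveCollection creates the root objective collection with ordered completion required.
; Populate Objectives adds one BP_ObjReachDestination per stop to that collection, each bound to its own trigger reference and owned by the quest.
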(fn ConstructionScript
  (|CallParentFunction))

(fn ConstructRootObjectiveCollection
  (bind _returnvalue (Game|ConstructObjectfromClass "/Game/QuestSystem/Objectives/BP_ObjCollection.BP_ObjCollection_C" self true "A Long Way Home"))
  (return _returnvalue))

(fn PopulateObjectives
  (params (RootObjCollection :type BP%20Obj%20Collection%20Object%20Reference))
  (Utilities|FlowControl|Sequence
    (:then_0
      (bind _returnvalue (Game|ConstructObjectfromClass "/Game/QuestSystem/Objectives/BP_ObjReachDestination.BP_ObjReachDestination_C" self (Variables|Default|GetGeekbrainsTrigger) "Reach GEEKBRAINS"))
      (Default|AddObjective RootObjCollection _returnvalue))
    (:then_1
      (bind _returnvalue_2 (Game|ConstructObjectfromClass "/Game/QuestSystem/Objectives/BP_ObjReachDestination.BP_ObjReachDestination_C" self (Variables|Default|GetSkillboxTrigger) "Reach SKILLBOX"))
      (Default|AddObjective RootObjCollection _returnvalue_2))
    (:then_2
      (bind _returnvalue_3 (Game|ConstructObjectfromClass "/Game/QuestSystem/Objectives/BP_ObjReachDestination.BP_ObjReachDestination_C" self (Variables|Default|GetNetologyTrigger) "Reach NETOLOGY"))
      (Default|AddObjective RootObjCollection _returnvalue_3))))