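; BP_ObjCollection is a composite quest objective that groups child objectives and counts as complete only when all of them are.
; On activation it calls the parent, then either activates every child at once or, when OrderRequired is set, only the first incomplete one.
; In ordered mode, each child's OnCompleted event unbinds itself, then activates and binds the next incomplete child, forming a sequential chain.
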(event Custom|OnCompleted_Event_0
  (params (Objective :type BP%20Objective%20Object%20Reference))
  (EventDispatchers|UnbindEventfromOnCompleted Objective (delegate Custom|OnCompleted_Event_0))
  (bind _nexobjective (Private|FindNextIncompleteObjective))
  (Utilities|IsValid _nexobjective
    (:Is%20Valid
      (Default|ActivateObjective _nexobjective)
      (EventDispatchers|AssignOnCompleted _nexobjective (delegate Custom|OnCompleted_Event_0)))))

(event EventActivateObjective
  (|CallParentFunction)
  (if (Variables|Default|GetOrderRequired)
    (bind _nexobjective (Private|FindNextIncompleteObjective))
    (Utilities|IsValid _nexobjective
      (:Is%20Valid
        (Default|ActivateObjective _nexobjective)
        (EventDispatchers|AssignOnCompleted _nexobjective (delegate Custom|OnCompleted_Event_0))))
    (else
      (for _array_element (Variables|Default|GetObjectives)
        (Default|ActivateObjective _array_element)))))

(fn FindNextIncompleteObjective
  (for _array_element (Variables|Default|GetObjectives)
    (bind _iscomplete (CallFunction|GetIsComplete _array_element))
    (if (not _iscomplete)
      (return _array_element)))
  (return 0))

(fn AddObjective
  (params (Objective :type BP%20Objective%20Object%20Reference%20%28by%20ref%29))
  (Utilities|Array|Add (Variables|Default|GetObjectives) Objective))

(fn GetIsComplete
  (for _array_element (Variables|Default|GetObjectives)
    (bind _iscomplete (CallFunction|GetIsComplete _array_element))
    (if (not _iscomplete)
      (return false)))
  (return true))